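; Base weapon Blueprint with first and third person meshes that plays an attached fire sound when shot and handles reloading.
; An empty magazine automatically starts a timed reload, as CanReload always returns true, and OnWeaponReloaded refills the ammo count.
; Construction applies one shared dynamic material instance to both meshes, whose AddedColor parameter turns blue during reload and white afterward.
; Debug prints mark the empty-magazine and reload-start events.
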(event Custom|OnWeaponReloaded
  (bind _magazinesize (Variables|Default|GetMagazineSize))
  (Variables|Default|SetCurrentBulletCount _magazinesize)
  (Variables|Default|SetIsReloading false)
  (CallFunction|HideIsReloading)
  (Class|ShooterWeapon|UpdateCurrentAmmo _magazinesize))

(event Custom|OnMagazineBecameEmpty
  (Development|PrintString "BP OnMagazineBecameEmpty" true true "(R=0.051401,G=0.590625,B=0.138080,A=1.000000)" -1.0)
  (bind _ret (CallFunction|CanReload))
  (if _ret
    (CallFunction|Reload)))

(event EventBeginPlay
  (EventDispatchers|BindEventtoMagazineBecameEmpty (delegate Custom|OnMagazineBecameEmpty)))

(event EventOnShot
  (Audio|SpawnSoundAttached "/Game/FilesFromFpsTemplate/Weapons/GrenadeLauncher/Audio/FirstPersonTemplateWeaponFire02.FirstPersonTemplateWeaponFire02" (Variables|Default|GetAudio%20Component%20Fire) "None" "0, 0, 0" "0, 0, 0" "KeepRelativeOffset" false 1.0 1.0 0.0 0 0))

(fn ConstructionScript
  (bind _firstpersonmesh (Variables|Default|GetFirstPersonMesh))
  (bind _returnvalue (Rendering|Material|CreateDynamicMaterialInstance _firstpersonmesh 0 (Rendering|Material|GetMaterial _firstpersonmesh 0) "None" :!class /Script/Engine.PrimitiveComponent))
  (bind _output_get (Variables|Default|SetfpDynamicMatInstance _returnvalue))
  (Utilities|FlowControl|Sequence
    (:then_0
      (Rendering|Material|SetMaterial (Variables|Default|GetFirstPersonMesh) 0 _output_get))
    (:then_1
      (Rendering|Material|SetMaterial (Variables|Default|GetThirdPersonMesh) 0 _output_get))))

(fn CanReload
  (return true))

(fn Reload
  (Development|PrintString "RELOAD STARTED" true true "(R=0.769792,G=0.114377,B=0.000000,A=1.000000)" -1.0)
  (Variables|Default|SetIsReloading true)
  (Utilities|Time|SetTimerbyEvent (EventDispatchers|CreateEvent :!event Custom|OnWeaponReloaded) (Variables|Default|GetReloadDuration))
  (CallFunction|ShowIsReloading))

(fn ShowIsReloading
  (Rendering|Material|SetColorParameterValueonMaterials (Variables|Default|GetFirstPersonMesh) "AddedColor" "(R=0.000000,G=0.046049,B=0.707293,A=1.000000)")
  (Rendering|Material|SetColorParameterValueonMaterials (Variables|Default|GetThirdPersonMesh) "AddedColor" "(R=0.000000,G=0.046049,B=0.707293,A=1.000000)"))

(fn HideIsReloading
  (Rendering|Material|SetColorParameterValueonMaterials (Variables|Default|GetFirstPersonMesh) "AddedColor" "(R=1.000000,G=1.000000,B=1.000000,A=1.000000)")
  (Rendering|Material|SetColorParameterValueonMaterials (Variables|Default|GetThirdPersonMesh) "AddedColor" "(R=1.000000,G=1.000000,B=1.000000,A=1.000000)"))