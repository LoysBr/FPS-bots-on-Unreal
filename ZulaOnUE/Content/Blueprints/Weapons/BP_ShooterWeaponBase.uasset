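; Base shooter weapon Blueprint that handles automatic reloading and sets up a dynamic material on the first-person mesh.
; When the magazine empties, it checks CanReload, which always returns true here, then flags reloading and starts a timer lasting ReloadDuration.
; ShowIsReloading and HideIsReloading are empty hooks, and debug prints mark the magazine and reload events.
; The construction script stores the material instance; its explicit SetMaterial call is disconnected.
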(event Custom|OnWeaponReloaded
  (Development|PrintString "BP OnWeaponReloaded" true true "(R=0.051401,G=0.590625,B=0.138080,A=1.000000)" -1.0))

(event Custom|OnMagazineBecameEmpty
  (Development|PrintString "BP OnMagazineBecameEmpty" true true "(R=0.051401,G=0.590625,B=0.138080,A=1.000000)" -1.0)
  (bind _ret (CallFunction|CanReload))
  (if _ret
    (CallFunction|Reload)))

(event EventBeginPlay
  (EventDispatchers|BindEventtoMagazineBecameEmpty (delegate Custom|OnMagazineBecameEmpty)))

(fn ConstructionScript
  (bind _firstpersonmesh (Variables|Default|GetFirstPersonMesh))
  (bind _returnvalue (Rendering|Material|CreateDynamicMaterialInstance _firstpersonmesh 0 (Rendering|Material|GetMaterial _firstpersonmesh 0) "None" :!class /Script/Engine.PrimitiveComponent))
  (bind _output_get (Variables|Default|SetFirstPersonDynamicMaterial _returnvalue)))

(fn CanReload
  (return true))

(fn Reload
  (Development|PrintString "RELOAD STARTED" true true "(R=0.769792,G=0.114377,B=0.000000,A=1.000000)" -1.0)
  (Variables|Default|SetIsReloading true)
  (Utilities|Time|SetTimerbyEvent (EventDispatchers|CreateEvent :!event Custom|OnWeaponReloaded) (Variables|Default|GetReloadDuration))
  (CallFunction|ShowIsReloading))

(fn ShowIsReloading)

(fn HideIsReloading)